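; BP_Ghost is a ghost actor that chases one player character and freezes while a second one, the scarer, faces it.
; On server Tick, sphere overlaps within its sight radius fill Target from the first character found and Scarer from the second.
; Once both are set, it moves toward Target with a swept, speed-scaled step unless a dot product check shows Scarer facing it.
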(event `self.ReceiveTick`
  (params (DeltaSeconds :type "Float (single-precision)"))
  (bind _returnvalue (`self.K2_GetActorLocation`))
  (bind _target (`self.Target`))
  (bind _scarer (`self.Scarer`))
  (`/Engine/EditorBlueprintResources/ActorMacros.Switch Has Authority`
    (:`Authority`
      (`/Engine/EditorBlueprintResources/StandardMacros.IsValid` _target
        (:`Is Valid`
          (`/Engine/EditorBlueprintResources/StandardMacros.IsValid` _scarer
            (:`Is Valid`
              (bind _returnvalue_2 (`self.GetDotProductTo` _scarer self))
              (if (not (>= _returnvalue_2 0.9))
                ;[1 1 1] Follow Target
                (`self.K2_SetActorLocation` (+ _returnvalue (* (`KismetMathLibrary.Normal` (- (`self.K2_GetActorLocation` _target) _returnvalue)) (* (`self.Speed`) DeltaSeconds))) true)))
            (:`Is Not Valid`
              ;[1 1 1] Find Scarer
              (bind (_outactors _returnvalue_3) (`KismetSystemLibrary.SphereOverlapActors_NEW` (`self.K2_GetActorLocation`) (`self.Sight Radius`) (`|MakeArray` "ObjectTypeQuery3" :!type "EngineTypes.EObjectTypeQuery Enum") "/Game/Blueprints/MyCharacter.MyCharacter_C"))
              (if _returnvalue_3
                (set `self.Scarer` (`KismetArrayLibrary.Array_Get` _outactors 1))))))
        (:`Is Not Valid`
          ;[1 1 1] Find Target
          (bind (_outactors_2 _returnvalue_4) (`KismetSystemLibrary.SphereOverlapActors_NEW` (`self.K2_GetActorLocation`) (`self.Sight Radius`) (`|MakeArray` "ObjectTypeQuery3" :!type "EngineTypes.EObjectTypeQuery Enum") "/Game/Blueprints/MyCharacter.MyCharacter_C"))
          (if _returnvalue_4
            (set `self.Target` (`KismetArrayLibrary.Array_Get` _outactors_2))))))))

(fn `UserConstructionScript`)