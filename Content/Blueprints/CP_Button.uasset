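; CP_Button is a pressure button Blueprint that responds to actors or components overlapping its Trigger component.
; Begin and end overlaps, handled only with authority, call the ButtonPressed and ButtonReleased events.
; Each event prints a debug string and sets the whole actor's relative location to a fixed lowered or raised position, rather than offsetting it from its placed location.
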(event `self.Trigger.OnComponentBeginOverlap`
  (params (OtherActor :type "Actor Object Reference") (OtherComp :type "PrimitiveComponent Object Reference") (OtherBodyIndex :type Integer))
  (`/Engine/EditorBlueprintResources/ActorMacros.Switch Has Authority`
    (:`Authority`
      (`self.ButtonPressed`))))

(event `self.Trigger.OnComponentEndOverlap`
  (params (OtherActor :type "Actor Object Reference") (OtherComp :type "PrimitiveComponent Object Reference") (OtherBodyIndex :type Integer))
  (`/Engine/EditorBlueprintResources/ActorMacros.Switch Has Authority`
    (:`Authority`
      (`self.ButtonReleased`))))

(event `ButtonPressed`
  (`KismetSystemLibrary.PrintString` "Pressed")
  (`self.SetActorRelativeLocation` (0.0 0.0 -10.0)))

(event `ButtonReleased`
  (`KismetSystemLibrary.PrintString` "Released")
  (`self.SetActorRelativeLocation` (0.0 0.0 10.0)))

(fn `UserConstructionScript`)