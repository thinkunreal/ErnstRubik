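; Player character Blueprint that fires a bullet actor on left mouse click in a networked game.
; The bullet class depends on network role: authority requests BP_FuseBullet, while remote requests BP_BombBullet.
; Both pass the class through ServerAttemptSpawnBombBullet to AttemptSpawnBullet, which spawns only on authority, just ahead of the character along its facing, unless colliding.
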(event `Key|LeftMouseButton`
  ;[1 1 1] Spawn Fuse Bullet on LMB
  (:`Pressed`
    (`/Engine/EditorBlueprintResources/ActorMacros.Switch Has Authority`
      (:`Authority`
        (`self.Server Attempt Spawn Bomb Bullet` "/Game/Blueprints/BP_FuseBullet.BP_FuseBullet_C"))
      (:`Remote`
        (`self.Server Attempt Spawn Bomb Bullet` "/Game/Blueprints/BP_BombBullet.BP_BombBullet_C")))))

(event `Server Attempt Spawn Bomb Bullet`
  (params (`Bullet Class` :type "Actor Class Reference"))
  ;[1 1 1] Server Spawn Bomb Bullet
  (`self.Attempt Spawn Bullet` `Bullet Class`))

(fn `Attempt Spawn Bullet`
  (params (`Bullet Class` :type "Actor Class Reference"))
  (`/Engine/EditorBlueprintResources/ActorMacros.Switch Has Authority`
    (:`Authority`
      (`|SpawnActorFromClass` `Bullet Class` (`KismetMathLibrary.MakeTransform` (+ (* (`self.GetActorForwardVector`) 200.0) (`self.K2_GetActorLocation`)) (`self.K2_GetActorRotation`) (1.0 1.0 1.0))))))

(fn `UserConstructionScript`)