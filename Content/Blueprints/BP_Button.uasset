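; Pressure button that signals a target Blueprint with ToggleMessage while at least one actor overlaps its trigger.
; The authority tracks overlapping actors, sending true and pressing on the first entry, false and releasing when the last one leaves.
; ButtonPressed and ButtonReleased play and reverse the Press timeline, which moves the button along Z and fades an orange emissive glow on its dynamic material, created in the construction script.
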(event `self.Trigger.OnComponentBeginOverlap`
  (params (OtherActor :type "Actor Object Reference") (OtherComp :type "PrimitiveComponent Object Reference") (OtherBodyIndex :type Integer))
  ;[1 1 1] Server Button Trigger
  (`/Engine/EditorBlueprintResources/ActorMacros.Switch Has Authority`
    (:`Authority`
      (if (not (`KismetArrayLibrary.Array_Contains` (`self.Overlapping Actors`) OtherActor))
        (`KismetArrayLibrary.Array_Add` (`self.Overlapping Actors`) OtherActor)
        (if (== 1 (`KismetArrayLibrary.Array_Length` (`self.Overlapping Actors`)))
          (message `/Game/Blueprints/BPI_Interactions.Toggle` (`self.Target Blueprint`) true)
          (`self.ButtonPressed`))))))

(event `self.Trigger.OnComponentEndOverlap`
  (params (OtherActor :type "Actor Object Reference") (OtherComp :type "PrimitiveComponent Object Reference") (OtherBodyIndex :type Integer))
  ;[1 1 1] Server Button Trigger
  (`/Engine/EditorBlueprintResources/ActorMacros.Switch Has Authority`
    (:`Authority`
      (`KismetArrayLibrary.Array_RemoveItem` (`self.Overlapping Actors`) OtherActor)
      (if (== 0 (`KismetArrayLibrary.Array_Length` (`self.Overlapping Actors`)))
        (message `/Game/Blueprints/BPI_Interactions.Toggle` (`self.Target Blueprint`) false)
        (`self.ButtonReleased`)))))

(event `ButtonPressed`
  ;[1 1 1] Client Visual Buttonstate
  (bind (_direction _press _glow) (`Timeline|Press` :!label _label)
    (:`Update`
      (`SceneComponent.SetRelativeLocation` (`self.Button`) (`KismetMathLibrary.MakeVector` 0.0 0.0 _press) false)
      (`MaterialInstanceDynamic.SetVectorParameterValue` (`self.Button material`) "Emissive" (`KismetMathLibrary.LinearColorLerp` (struct) (struct :`R` 0.6 :`G` 0.329323 :`A` 1.0) _glow)))))

(event `ButtonReleased`
  ;[1 1 1] Client Visual Buttonstate
  (goto _label :!via `Reverse`))

(fn `UserConstructionScript`
  (bind _returnvalue (`PrimitiveComponent.CreateDynamicMaterialInstance` (`self.Button`) 0 null))
  (set `self.Button material` _returnvalue))