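; ButtonStateLight is an actor that switches on while at least two toggle inputs are active and shows this with a spinning mesh.
; Toggle runs its logic only on authority, counting on signals up and off signals down, then sets Onoff from whether the count reaches two.
; While Onoff is true, Tick yaws StaticMesh1 at RotationSpeed scaled by delta time.
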(event `self.Toggle`
  (params (`On/off` :type Boolean))
  (`/Engine/EditorBlueprintResources/ActorMacros.Switch Has Authority`
    (:`Authority`
      (if `On/off`
        (set `self.ToggleCounter` (+ (`self.ToggleCounter`) 1))
        (else
          (set `self.ToggleCounter` (- (`self.ToggleCounter`) 1))))
      (set `self.On/off` (>= (`self.ToggleCounter`) 2)))))

(event `self.ReceiveTick`
  (params (DeltaSeconds :type "Float (single-precision)"))
  (if (`self.On/off`)
    (`SceneComponent.AddLocalRotation` (`self.StaticMesh1`) (`KismetMathLibrary.MakeRot` 0.0 (* DeltaSeconds (`self.Rotation Speed`))) false)))

(fn `UserConstructionScript`)