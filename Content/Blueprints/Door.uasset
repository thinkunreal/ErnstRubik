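; Door Blueprint that swings open once a toggle counter reaches a threshold of two.
; Toggle runs only on the authority, adjusting the counter and setting an on/off flag that triggers OpenDoor.
; OpenDoor plays a timeline that drives the door's relative yaw, then disables its collision when finished; no closing path exists.
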(event `self.Toggle`
  (params (`On/off` :type Boolean))
  (`/Engine/EditorBlueprintResources/ActorMacros.Switch Has Authority`
    (:`Authority`
      (if (not (`self.On/off`))
        (if `On/off`
          (set `self.ToggleCounter` (+ (`self.ToggleCounter`) 1))
          (else
            (set `self.ToggleCounter` (- (`self.ToggleCounter`) 1))))
        (set `self.On/off` (>= (`self.ToggleCounter`) 2))
        (if (`self.On/off`)
          (`self.OpenDoor`))))))

(event `OpenDoor`
  (bind (_direction _dooryaw) (`Timeline|DoorOpen`)
    (:`Update`
      (`SceneComponent.SetRelativeRotation` (`self.Door`) (`KismetMathLibrary.MakeRot` 0.0 _dooryaw) false))
    (:`Finished`
      (`PrimitiveComponent.SetCollisionEnabled` (`self.Door`) "NoCollision"))))

(fn `UserConstructionScript`)